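; PC_Lobby is the lobby player controller, which sets up the lobby UI for the local player.
; On BeginPlay it creates the W_lobby widget with UI-only input and a visible cursor; its construction script copies the pilot name from GI_Main.
; Events refresh the HUD's display settings and forward ready requests to PS_Lobby.
; The player-list and player-ready update events are empty, leaving some HUD update logic disconnected.
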(event Custom|update_settings
  (Default|UpdateDisplaySettings (Variables|Default|GetHUD)))

(event Custom|update_player_ready
  (params (player_state :type PS%20Lobby%20Object%20Reference)))

(event Custom|player%20ready
  (bind _asps_lobby (Utilities|Casting|CastToPS_Lobby (Variables|GetPlayerState self)))
  (Default|PlayerStateReady _asps_lobby))

(event Custom|update_player_list
  (params (login%20out :type Boolean) (Players :type Array%20of%20PC%20Lobby%20Object%20References)))

(event EventBeginPlay
  (bind _returnvalue (Game|GetPlayerController 0))
  (if (Pawn|IsLocalPlayerController)
    (bind _returnvalue_2 (UserInterface|CreateWidget "/Game/Server/Lobby/W_lobby.W_lobby_C"))
    (bind _output_get (Variables|Default|SetHUD _returnvalue_2))
    (UserInterface|Viewport|AddtoViewport _output_get 0)
    (Input|SetInputModeUIOnly _returnvalue _output_get "DoNotLock" false)
    (Variables|/Script/Engine.PlayerController|SetbShowMouseCursor _returnvalue true)))

(fn ConstructionScript
  (if (Pawn|IsLocalPlayerController)
    (bind _asgi_main (Utilities|Casting|CastToGI_Main (Game|GetGameInstance)))
    (Variables|Default|Setpilot_name (Variables|/Game/GI_Main.GI_Main_C|Getpilot_name _asgi_main))))