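; Lobby game mode that registers joining players and hands player-list updates to the lobby game state.
; PostLogin adds each PC_Lobby to a unique Players array and passes it to GS_lobby.AddNewPlayer, while refresh_lists calls GS_lobby.UpdatePlayers.
; Logout does nothing, as the removal logic and the older per-controller list broadcast are disconnected, so departed players stay in Players.
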(event Custom|refresh_lists
  (params (login%20out :type Boolean))
  (bind _asgs_lobby (Utilities|Casting|CastToGS_lobby (Game|GetGameState)))
  (Default|UpdatePlayers _asgs_lobby))

(event EventPostLogin
  (params (NewPlayer :type Player%20Controller%20Object%20Reference))
  (bind _aspc_lobby (Utilities|Casting|CastToPC_Lobby NewPlayer))
  (Utilities|Array|AddUnique (Variables|Default|Getplayers) _aspc_lobby)
  (bind _asgs_lobby (Utilities|Casting|CastToGS_lobby (Game|GetGameState)))
  (Default|AddNewPlayer _asgs_lobby _aspc_lobby))

(event EventOnLogout
  (params (ExitingController :type Controller%20Object%20Reference)))

(fn ConstructionScript)