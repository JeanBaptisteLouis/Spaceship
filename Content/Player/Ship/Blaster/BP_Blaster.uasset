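; Ship-mounted blaster component that auto-fires BP_laser projectiles from its location toward the owning ship's ShootTarget, using the ship's bullet speed.
; Start and stop events drive a looping timer that calls Shoot.
; Shoot spawns a laser immediately, then relays the rotation through a server, all, local event chain.
; A HasShot flag swallows the echoed shot on the firer, so only other instances spawn that laser.
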(event Custom|Shoot
  (bind _returnvalue (Transformation|GetWorldLocation))
  (bind _ship (Variables|Default|Getship))
  (bind _shoot_target (Variables|/Game/Player/Ship/Pawn/BP_Ship.BP_ship_C|Getshoot_target _ship))
  (bind _returnvalue_2 (- _shoot_target _returnvalue))
  (bind _returnvalue_3 (Math|Conversions|RotationFromXVector _returnvalue_2))
  (Utilities|FlowControl|Sequence
    (:then_0
      (Game|SpawnActorfromClass "/Game/Player/Ship/Blaster/BP_laser.BP_laser_C" (Math|Transform|MakeTransform _returnvalue _returnvalue_3 "1.000000,1.000000,1.000000") "AlwaysSpawn" "MultiplyWithRoot" 0 (Variables|/Game/Player/Ship/Pawn/BP_Ship.BP_ship_C|Getbullet_speed (Variables|Default|Getship)) (Variables|Default|Getship) 0)
      (Variables|Default|Sethas_shot true))
    (:then_1
      (CallFunction|ShootServ _returnvalue_3))))

(event Custom|Shoot_serv
  (params (Spawn%20Transform%20Rotation :type Rotator))
  (CallFunction|ShootAll Spawn%20Transform%20Rotation))

(event Custom|stopShooting
  (Utilities|Time|ClearandInvalidateTimerbyHandle (stale Custom|startShooting _returnvalue)))

(event Custom|startShooting
  (bind _returnvalue (Utilities|Time|SetTimerbyEvent (delegate Custom|Shoot) 0.14 true -0.14)))

(event Custom|shoot_all
  (params (Spawn%20Transform%20Rotation :type Rotator))
  (CallFunction|ShootLocal Spawn%20Transform%20Rotation))

(event Custom|shoot_local
  (params (Spawn%20Transform%20Rotation :type Rotator))
  (if (Variables|Default|Gethas_shot)
    (Variables|Default|Sethas_shot false)
    (else
      (Game|SpawnActorfromClass "/Game/Player/Ship/Blaster/BP_laser.BP_laser_C" (Math|Transform|MakeTransform (Transformation|GetWorldLocation) Spawn%20Transform%20Rotation "1.000000,1.000000,1.000000") "AlwaysSpawn" "MultiplyWithRoot" 0 (Variables|/Game/Player/Ship/Pawn/BP_Ship.BP_ship_C|Getbullet_speed (Variables|Default|Getship)) (Variables|Default|Getship) 0))))

(event EventBeginPlay
  (bind _asbp_ship (Utilities|Casting|CastToBP_ship (Components|GetOwner)))
  (Variables|Default|Setship _asbp_ship))

(event EventTick
  (params (DeltaSeconds :type Float%20%28single-precision%29)))