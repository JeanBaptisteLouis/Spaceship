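; Combat component for the player ship that tracks Health, deals and receives damage, and destroys its owner at zero health.
; Hits reach the target through its combat message object, fetched via GetCombatCompMessage, passing the owner as damage author.
; A lethal hit notifies the killer through the same message route.
; Kill and death events are reported to player state index 0, not one resolved from the owner.
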(event Custom|Die
  (Actor|DestroyActor (Components|GetOwner)))

(event Custom|receive_damage
  (params (author :type Actor%20Object%20Reference) (amount :type Float%20%28double-precision%29))
  (Variables|Default|Sethealth (- (Variables|Default|Gethealth) amount))
  (Development|PrintString "hit")
  (if (<= (Variables|Default|Gethealth) 0.0)
    (bind _comp (Class|BPICombat|GetCombatComp(Message) author))
    (Class|BPICombatMain|HasKilled(Message) _comp (Components|GetOwner))
    (CallFunction|HasBeenKilled author)
    (CallFunction|Die)))

(event Custom|sendDamage
  (params (hit_actor :type Actor%20Object%20Reference) (amount :type Float%20%28double-precision%29))
  (bind _comp (Class|BPICombat|GetCombatComp(Message) hit_actor))
  (Utilities|IsValid _comp
    (:Is%20Valid
      (CallFunction|ReceiveDamage _comp (Components|GetOwner) amount))))

(event Custom|callDeath
  (params (author :type Actor%20Object%20Reference))
  (Class|BPIPS|Death(Message) (Game|GetPlayerState 0) author))

(event Custom|callKill
  (params (victim :type Actor%20Object%20Reference))
  (Class|BPIPS|Kill(Message) (Game|GetPlayerState 0) victim))

(event EventHit
  (params (hit_actor :type Actor%20Object%20Reference) (amount :type Float%20%28double-precision%29))
  (CallFunction|SendDamage hit_actor amount))

(event EventHasBeenKilled
  (params (author :type Actor%20Object%20Reference))
  (CallFunction|CallDeath author))

(event EventHasKilled
  (params (victim :type Actor%20Object%20Reference))
  (CallFunction|CallKill victim))