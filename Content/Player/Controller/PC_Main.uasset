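; Main player controller that switches the player between a map overview spawn screen and piloting a ship.
; Spawn and initialization requests route through server events, while possession and the PossessedPawn OnRep update the pawn, swapping Enhanced Input mapping contexts, input mode and cursor.
; Ship input actions are forwarded to the possessed ship.
; A ship-destroyed handler returns possession to the overview pawn.
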(event Custom|Switch%20control%20mode
  (params (new%20mode :type ENUM_control_modes%20Enum :default "NewEnumerator0"))
  (bind _returnvalue (Utilities|Select :Index new%20mode :NewEnumerator0 "/Game/Player/Controller/Inputs/IMC_Spawn.IMC_Spawn" :NewEnumerator1 "/Game/Player/Controller/Inputs/IMC_Ship.IMC_Ship" :NewEnumerator2 0))
  (Input|RemoveMappingContext (PlayerController|LocalPlayerSubsystems|GetEnhancedInputLocalPlayerSubsystem self) (Variables|Default|Getcurrent%20mapping%20context) "(bIgnoreAllPressedKeysUntilRelease=True,bForceImmediately=False,bNotifyUserSettings=False)")
  (Input|AddMappingContext (PlayerController|LocalPlayerSubsystems|GetEnhancedInputLocalPlayerSubsystem self) _returnvalue 0 "(bIgnoreAllPressedKeysUntilRelease=True,bForceImmediately=False,bNotifyUserSettings=False)")
  (Variables|Default|Setcurrent%20mapping%20context _returnvalue))

(event Custom|SpawnCallOnServer
  (params (SP :type BP%20Spawn%20Point%20Object%20Reference))
  (Default|CallSpawn self SP))

(event Custom|SpawnCall
  (params (SP :type BP%20Spawn%20Point%20Object%20Reference))
  (CallFunction|SpawnCallonServer SP))

(event Custom|ShipDestroyed
  (bind _overview_ref (Variables|Default|GetOverview_ref)
    (:then
      (Pawn|Possess _overview_ref))
    (:else)))

(event Custom|CallInitializeOnServer
  (Default|CallInitialize self))

(event Custom|updatePawn
  (bind _possessed_pawn (Variables|Default|GetPossessed%20Pawn))
  (bind _asbp_ship (Utilities|Casting|CastToBP_ship _possessed_pawn)
    (:then
      (bind _output_get (Variables|Default|SetShip_ref _asbp_ship))
      (CallFunction|SwitchControlMode "NewEnumerator1")
      (EventDispatchers|BindEventtoDestroyed _output_get (EventDispatchers|CreateEvent :!event Custom|ShipDestroyed))
      (CallFunction|UpdateHUD "NewEnumerator1"))
    (:CastFailed
      (bind _asbp_map_overview (Utilities|Casting|CastToBP_MapOverview _possessed_pawn))
      (Variables|Default|SetOverview_ref _asbp_map_overview)
      (CallFunction|SwitchControlMode "NewEnumerator0")
      (CallFunction|UpdateHUD "NewEnumerator0"))))

(event Custom|updateHUD
  (params (mode :type ENUM_control_modes%20Enum :default "NewEnumerator0"))
  (bind _self self)
  (bind _self_2 self)
  (switch Utilities|FlowControl|Switch|SwitchonENUM_control_modes mode
    (:NewEnumerator0
      (bind _returnvalue (UserInterface|CreateWidget "/Game/Server/Overview/W_Overview.W_Overview_C" self))
      (UserInterface|Viewport|AddtoViewport _returnvalue 0)
      (Input|SetInputModeUIOnly _self_2 _returnvalue "DoNotLock" false)
      (Variables|/Script/Engine.PlayerController|SetbShowMouseCursor _self_2 true))
    (:NewEnumerator1
      (Input|SetInputModeGameOnly _self false)
      (Variables|/Script/Engine.PlayerController|SetbShowMouseCursor _self false))))

(event Input|EnhancedActionEvents|EnhancedInputActionIA_Look
  (params (ActionValue :type Vector%202D%20Structure) (ElapsedSeconds :type Float%20%28double-precision%29) (TriggeredSeconds :type Float%20%28double-precision%29) (InputAction :type Input%20Action%20Object%20Reference :default "/Game/Player/Controller/Inputs/Actions/IA_Look.IA_Look"))
  ;[1 1 1] Ship controls
  (bind _ship_ref (Variables|Default|GetShip_ref)
    (:then
      (Default|InputLook _ship_ref ActionValue))
    (:else)))

(event Input|EnhancedActionEvents|EnhancedInputActionIA_Roll
  (params (ActionValue :type Float%20%28double-precision%29) (ElapsedSeconds :type Float%20%28double-precision%29) (TriggeredSeconds :type Float%20%28double-precision%29) (InputAction :type Input%20Action%20Object%20Reference :default "/Game/Player/Controller/Inputs/Actions/IA_Roll.IA_Roll"))
  ;[1 1 1] Ship controls
  (bind _ship_ref (Variables|Default|GetShip_ref)
    (:then
      (Default|InputRoll _ship_ref ActionValue))
    (:else)))

(event Input|EnhancedActionEvents|EnhancedInputActionIA_FwBw
  (params (ActionValue :type Float%20%28double-precision%29) (ElapsedSeconds :type Float%20%28double-precision%29) (TriggeredSeconds :type Float%20%28double-precision%29) (InputAction :type Input%20Action%20Object%20Reference :default "/Game/Player/Controller/Inputs/Actions/IA_FwBw.IA_FwBw"))
  ;[1 1 1] Ship controls
  (bind _ship_ref (Variables|Default|GetShip_ref)
    (:then
      (Default|InputForward _ship_ref ActionValue))
    (:else)))

(event Input|EnhancedActionEvents|EnhancedInputActionIA_Horizontal
  (params (ActionValue :type Float%20%28double-precision%29) (ElapsedSeconds :type Float%20%28double-precision%29) (TriggeredSeconds :type Float%20%28double-precision%29) (InputAction :type Input%20Action%20Object%20Reference :default "/Game/Player/Controller/Inputs/Actions/IA_Horizontal.IA_Horizontal"))
  ;[1 1 1] Ship controls
  (bind _ship_ref (Variables|Default|GetShip_ref)
    (:then
      (Default|InputHorizontal _ship_ref ActionValue))
    (:else)))

(event Input|EnhancedActionEvents|EnhancedInputActionIA_Vertical
  (params (ActionValue :type Float%20%28double-precision%29) (ElapsedSeconds :type Float%20%28double-precision%29) (TriggeredSeconds :type Float%20%28double-precision%29) (InputAction :type Input%20Action%20Object%20Reference :default "/Game/Player/Controller/Inputs/Actions/IA_Vertical.IA_Vertical"))
  ;[1 1 1] Ship controls
  (bind _ship_ref (Variables|Default|GetShip_ref)
    (:then
      (Default|InputVertical _ship_ref ActionValue))
    (:else)))

(event Input|EnhancedActionEvents|EnhancedInputActionIA_Brake
  (params (ActionValue :type Boolean) (ElapsedSeconds :type Float%20%28double-precision%29) (TriggeredSeconds :type Float%20%28double-precision%29) (InputAction :type Input%20Action%20Object%20Reference :default "/Game/Player/Controller/Inputs/Actions/IA_Brake.IA_Brake"))
  ;[1 1 1] Ship controls
  (bind _ship_ref (Variables|Default|GetShip_ref)
    (:then
      (Default|InputBrake _ship_ref))
    (:else)))

(event Input|EnhancedActionEvents|EnhancedInputActionIA_Shoot
  (params (ActionValue :type Boolean) (ElapsedSeconds :type Float%20%28double-precision%29) (TriggeredSeconds :type Float%20%28double-precision%29) (InputAction :type Input%20Action%20Object%20Reference :default "/Game/Player/Controller/Inputs/Actions/IA_Shoot.IA_Shoot"))
  ;[1 1 1] Ship controls
  (bind _ship_ref (Variables|Default|GetShip_ref)
    (:then
      (Default|InputShoot _ship_ref ActionValue))
    (:else)))

(event EventBeginPlay
  (CallFunction|CallInitializeonServer)
  (if (Pawn|IsLocalPlayerController)
    _))

(event EventPossess
  (params (PossessedPawn :type Pawn%20Object%20Reference))
  (Variables|Default|SetPossessed%20Pawn PossessedPawn)
  (CallFunction|UpdatePawn))

(fn ConstructionScript)

(fn OnRepPossessedPawn
  (CallFunction|UpdatePawn)
  (Development|PrintString "Hello"))